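; BP_NPCSpawner is an actor that supplies hotel NPCs one at a time from a daily quota.
; RequestNextNPC spawns a BP_HotelNPC at the spawner's transform with a random skeletal mesh, decrements the count and returns Japanese remaining-count text.
; It relays the current NPC's arrival through OnNPCArrived, while PassNPC tells that NPC to enter.
; OnReset destroys the current NPC and restores the quota.
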(event Custom|OnNPCSubscribed
  (EventDispatchers|BindEventtoOnArrived (Variables|Default|GetCurrentNPC) (delegate Custom|OnArrive)))

(event Custom|OnArrive
  (Default|CallOnNPCArrived))

(event Custom|OnReset
  (CallFunction|KillNPC)
  (Variables|Default|SetMaxTodayNPCCount 3)
  (Variables|Default|SetCurrentNPCCount (Variables|Default|GetMaxTodayNPCCount)))

(event EventBeginPlay
  (Variables|Default|SetCurrentNPCCount (Variables|Default|GetMaxTodayNPCCount)))

(event Collision|EventActorBeginOverlap
  (params (OtherActor :type Actor%20Object%20Reference)))

(event EventTick
  (params (DeltaSeconds :type Float%20%28single-precision%29)))

(fn ConstructionScript)

(fn RequestNextNPC
  (if (<= (Variables|Default|GetCurrentNPCCount) 0)
    (return (Utilities|Text|FormatText "残り: [0/{MaxCount}名]" (Variables|Default|GetMaxTodayNPCCount)))
    (else
      (bind _returnvalue (Game|SpawnActorfromClass "/Game/Blueprint/BP_HotelNPC.BP_HotelNPC_C" (Transformation|GetActorTransform) "Undefined" "MultiplyWithRoot" 0 0))
      (bind _output_get (Variables|Default|SetCurrentNPC _returnvalue))
      (Components|SkeletalMesh|SetSkeletalMeshAsset (Variables|/Script/Engine.Character|GetMesh _output_get) (.OutItem (Utilities|Array|Random (Variables|Default|GetSkeletalMeshes))))
      (CallFunction|OnNPCSubscribed)
      (bind _output_get_2 (Variables|Default|SetCurrentNPCCount (- (Variables|Default|GetCurrentNPCCount) 1)))
      (return (Utilities|Text|FormatText "残り: [{0}/{1}名]" (+ _output_get_2 1) (Variables|Default|GetMaxTodayNPCCount))))))

(fn PassNPC
  (Default|NPCEnter (Variables|Default|GetCurrentNPC)))

(fn KillNPC
  (bind _currentnpc (Variables|Default|GetCurrentNPC))
  (Utilities|IsValid _currentnpc
    (:Is%20Valid
      (Actor|DestroyActor _currentnpc))))

(fn HasNextNPC
  (return (> (Variables|Default|GetCurrentNPCCount) 0)))