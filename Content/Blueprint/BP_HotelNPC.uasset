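; BP_HotelNPC is a hotel NPC character that walks a set distance forward, then turns to face the player's camera.
; BeginPlay records the start location and applies MoveSpeed, and Tick adds forward movement input until TargetDistance is reached.
; It then stops and smoothly interpolates toward the camera with RInterpTo.
; Once yaw is within one degree, HasRotated latches, so it does not keep tracking the camera.
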(event EventBeginPlay
  (Variables|Default|SetIsMoving true)
  (Variables|Default|SetStartLocation (Transformation|GetActorLocation))
  (Variables|/Script/Engine.CharacterMovementComponent|SetMaxWalkSpeed (Variables|Character|GetCharacterMovement) (Variables|Default|GetMoveSpeed)))

(event Collision|EventActorBeginOverlap
  (params (OtherActor :type Actor%20Object%20Reference)))

(event EventTick
  (params (DeltaSeconds :type Float%20%28single-precision%29))
  (bind _returnvalue (Transformation|GetActorLocation))
  (bind _returnvalue_2 (Transformation|GetActorRotation))
  (bind _returnvalue_3 (Game|GetPlayerCameraManager 0))
  (bind _returnvalue_4 (Camera|GetCameraLocation _returnvalue_3))
  (bind _returnvalue_5 (Math|Rotator|FindLookatRotation _returnvalue _returnvalue_4))
  (if (Variables|Default|GetIsMoving)
    (Pawn|Input|AddMovementInput (Transformation|GetActorForwardVector) 1.0 false)
    (if (>= (Math|Vector|Distance(Vector) (Variables|Default|GetStartLocation) (Transformation|GetActorLocation)) (Variables|Default|GetTargetDistance))
      (Variables|Default|SetIsMoving false)
      (Components|Movement|StopMovementImmediately (Variables|Character|GetCharacterMovement)))
    (elif (not (Variables|Default|GetHasRotated))
      (Transformation|SetActorRotation (Math|Interpolation|RInterpTo _returnvalue_2 _returnvalue_5 (Utilities|Time|GetWorldDeltaSeconds) 5.0))
      (if (< (Math|Float|Absolute(Float) (.Yaw (Math|Rotator|BreakRotator (Math|Rotator|Delta(Rotator) _returnvalue_2 _returnvalue_5)))) 1.0)
        (Variables|Default|SetHasRotated true)))))

(fn ConstructionScript)